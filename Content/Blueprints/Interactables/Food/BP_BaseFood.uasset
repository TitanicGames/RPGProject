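; Base Blueprint for food items that restore the eating character's health, stamina and/or magic.
; The Eat event stores the instigating character, then switches on the food type in FoodInfo to choose which attributes to restore.
; One restore function per attribute adds the FoodInfo amount directly to that character's current value, capped at its maximum.
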(event Custom|Eat
  (params (Instigator :type CH%20My%20Character%20Object%20Reference))
  ;[1 1 1] Restore the specified attributes when Eat is called. Eat is called from the character when a Food item is used.
  (Variables|Default|SetCharacterReference Instigator)
  (switch Utilities|FlowControl|Switch|SwitchonEFoodType (Utilities|Struct|BreakFFoodInfo (Variables|Default|GetFoodInfo))
    (:NewEnumerator0
      (CallFunction|RestoreHealth))
    (:NewEnumerator1
      (CallFunction|RestoreStamina))
    (:NewEnumerator2
      (CallFunction|RestoreMagic))
    (:NewEnumerator3
      (CallFunction|RestoreHealth)
      (CallFunction|RestoreStamina))
    (:NewEnumerator4
      (CallFunction|RestoreHealth)
      (CallFunction|RestoreMagic))
    (:NewEnumerator5
      (CallFunction|RestoreStamina)
      (CallFunction|RestoreMagic))
    (:NewEnumerator6
      (CallFunction|RestoreHealth)
      (CallFunction|RestoreStamina)
      (CallFunction|RestoreMagic))))

(fn ConstructionScript
  (|CallParentFunction))

(fn RestoreHealth
  (bind _characterreference (Variables|Default|GetCharacterReference))
  (bind _characterreference_2 (Variables|Default|GetCharacterReference))
  (bind _maxhealth (Variables|/Game/Blueprints/Game/CH_MyCharacter.CH_MyCharacter_C|GetMaxHealth _characterreference_2))
  (if (> (+ (Utilities|Struct|BreakFFoodInfo (Variables|Default|GetFoodInfo)) (Variables|/Game/Blueprints/Game/CH_MyCharacter.CH_MyCharacter_C|GetCurrentHealth _characterreference_2)) _maxhealth)
    (Variables|/Game/Blueprints/Game/CH_MyCharacter.CH_MyCharacter_C|SetCurrentHealth _characterreference _maxhealth)
    (else
      (Variables|/Game/Blueprints/Game/CH_MyCharacter.CH_MyCharacter_C|SetCurrentHealth _characterreference (+ (Utilities|Struct|BreakFFoodInfo (Variables|Default|GetFoodInfo)) (Variables|/Game/Blueprints/Game/CH_MyCharacter.CH_MyCharacter_C|GetCurrentHealth _characterreference_2))))))

(fn RestoreStamina
  (bind _characterreference (Variables|Default|GetCharacterReference))
  (bind _characterreference_2 (Variables|Default|GetCharacterReference))
  (bind _maxstamina (Variables|/Game/Blueprints/Game/CH_MyCharacter.CH_MyCharacter_C|GetMaxStamina _characterreference_2))
  (if (> (+ (Utilities|Struct|BreakFFoodInfo (Variables|Default|GetFoodInfo)) (Variables|/Game/Blueprints/Game/CH_MyCharacter.CH_MyCharacter_C|GetCurrentStamina _characterreference_2)) _maxstamina)
    (Variables|/Game/Blueprints/Game/CH_MyCharacter.CH_MyCharacter_C|SetCurrentStamina _characterreference _maxstamina)
    (else
      (Variables|/Game/Blueprints/Game/CH_MyCharacter.CH_MyCharacter_C|SetCurrentStamina _characterreference (+ (Utilities|Struct|BreakFFoodInfo (Variables|Default|GetFoodInfo)) (Variables|/Game/Blueprints/Game/CH_MyCharacter.CH_MyCharacter_C|GetCurrentStamina _characterreference_2))))))

(fn RestoreMagic
  (bind _characterreference (Variables|Default|GetCharacterReference))
  (bind _characterreference_2 (Variables|Default|GetCharacterReference))
  (bind _maxmagic (Variables|/Game/Blueprints/Game/CH_MyCharacter.CH_MyCharacter_C|GetMaxMagic _characterreference_2))
  (if (> (+ (Utilities|Struct|BreakFFoodInfo (Variables|Default|GetFoodInfo)) (Variables|/Game/Blueprints/Game/CH_MyCharacter.CH_MyCharacter_C|GetCurrentMagic _characterreference_2)) _maxmagic)
    (Variables|/Game/Blueprints/Game/CH_MyCharacter.CH_MyCharacter_C|SetCurrentMagic _characterreference _maxmagic)
    (else
      (Variables|/Game/Blueprints/Game/CH_MyCharacter.CH_MyCharacter_C|SetCurrentMagic _characterreference (+ (Utilities|Struct|BreakFFoodInfo (Variables|Default|GetFoodInfo)) (Variables|/Game/Blueprints/Game/CH_MyCharacter.CH_MyCharacter_C|GetCurrentMagic _characterreference_2))))))